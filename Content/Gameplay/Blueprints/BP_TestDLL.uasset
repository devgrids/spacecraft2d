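; Test Blueprint that exercises loading a native DLL, idroy.dll, from the Plugins folder at runtime.
; On BeginPlay it loads the library, then imports bool-inversion, integer-increment and circle-area functions in sequence.
; It calls the bool and circle-area functions and prints results or failure messages, while the increment function is only imported.
; EndPlay frees the DLL.
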(event EventBeginPlay
  (bind _returnvalue (Class|CreateandLinkDLLTutBFL|ImportDLL "Plugins" "idroy.dll"))
  (if _returnvalue
    (Utilities|FlowControl|Sequence
      (:then_0
        (bind _returnvalue_2 (Class|CreateandLinkDLLTutBFL|ImportMethodGetInvertedBool))
        (if _returnvalue_2
          (bind _returnvalue_3 (Class|CreateandLinkDLLTutBFL|GetInvertedBoolfromDll false))
          (Development|PrintString (Utilities|String|Append "The inverted bool is: " (Utilities|String|ToString(Boolean) _returnvalue_3)))
          (else
            (Development|PrintString "Failed impor get invert bool"))))
      (:then_1
        (Class|CreateandLinkDLLTutBFL|ImportMethodGetIntPlusPlus))
      (:then_2
        (bind _returnvalue_4 (Class|CreateandLinkDLLTutBFL|ImportMethodGetCircleArea))
        (if _returnvalue_4
          (bind _returnvalue_5 (Class|CreateandLinkDLLTutBFL|GetCircleAreafromDll 15.0))
          (Development|PrintString (Utilities|String|Append "The circle area is: " (Utilities|String|ToString(Float) _returnvalue_5)))
          (else
            (Development|PrintString "Failed impor get invert bool")))))
    (else
      (Development|PrintString "DLL Failed"))))

(event EventEndPlay
  (params (EndPlayReason :type EEndPlayReason%20Enum :default "Destroyed"))
  (Class|CreateandLinkDLLTutBFL|FreeDLL))

(fn ConstructionScript)