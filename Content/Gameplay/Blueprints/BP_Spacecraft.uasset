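; BP_Spacecraft is a spacecraft Blueprint with a sprite component, holding only debug output and no gameplay logic.
; Key 1 prints the viewport width and height, and key 2 prints a zero vector.
; Overlaps on the sprite component print the attach parent socket name.
; Tick and the construction script are empty, and a print of sprite velocity magnitude is left unconnected.
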(event OnComponentBeginOverlap(SpriteComponent)
  (params (OverlappedComponent :type Primitive%20Component%20Object%20Reference) (OtherActor :type Actor%20Object%20Reference) (OtherComp :type Primitive%20Component%20Object%20Reference) (OtherBodyIndex :type Integer) (bFromSweep :type Boolean) (SweepResult :type Hit%20Result%20Structure%20%28by%20ref%29))
  (Development|PrintString (Utilities|String|ToString(Name) (Class|Actor|GetAttachParentSocketName))))

(event EventTick
  (params (DeltaSeconds :type Float%20%28single-precision%29)))

(event Input|KeyboardEvents|1
  (params (Key :type Key%20Structure :default "None"))
  (bind _returnvalue (Game|GetPlayerController 0))
  (bind (_sizex _sizey) (HUD|GetViewportSize _returnvalue))
  (:Pressed
    (Development|PrintString (Utilities|String|ToString(Integer) _sizex))
    (Development|PrintString (Utilities|String|ToString(Integer) _sizey))))

(event Input|KeyboardEvents|2
  (params (Key :type Key%20Structure :default "None"))
  (:Pressed
    (Development|PrintString (Utilities|String|ToString(Vector) "0, 0, 0") true true "(R=0.000000,G=0.660000,B=1.000000,A=1.000000)" 1e+01)))

(fn ConstructionScript)